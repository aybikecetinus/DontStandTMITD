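; BP_Door is a secret passage door that swings open and closed through custom open and close events.
; It caches the static mesh's world rotation at BeginPlay.
; GeçişTimeline supplies a Zaxis yaw offset, which is combined with that cached rotation and applied to the mesh on each update.
; Opening plays the timeline forward, and closing reverses it.
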(event `self.ReceiveBeginPlay`
  (set `self.DefaultRotation` (`SceneComponent.K2_GetComponentRotation` (`self.StaticMeshComponent`))))

(event `OpenSecretGeçiş`
  (bind (_direction _zaxis) (`Timeline|Geçiş Timeline` :!label _label)
    (:`Update`
      (`SceneComponent.K2_SetWorldRotation` (`self.StaticMeshComponent`) (`KismetMathLibrary.ComposeRotators` (`KismetMathLibrary.MakeRotator` 0.0 0.0 _zaxis) (`self.DefaultRotation`)) false false))))

(event `CloseSecretGeçiş`
  (goto _label :!via `Reverse`))

(fn `UserConstructionScript`)