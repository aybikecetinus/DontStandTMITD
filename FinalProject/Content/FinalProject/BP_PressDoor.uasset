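; BP_PressDoor is a door actor that moves to EndLocation when OpenPressDoor is triggered.
; It records its start location on BeginPlay, and OpenPressDoor enables Tick, which lerps between start and end without sweep.
; CurrentTime is set to DeltaSeconds plus RotationTime rather than accumulated, so with a positive RotationTime the alpha exceeds one immediately and Tick disables itself after one step.
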(event `self.ReceiveBeginPlay`
  (set `self.StartLocation` (`self.K2_GetActorLocation`)))

(event `/Game/FinalProject/PressDoorInterface.OpenPressDoor`
  (`self.SetActorTickEnabled` true))

(event `self.ReceiveTick`
  (params (DeltaSeconds :type "Float (single-precision)"))
  (set `self.Current Time` (+ DeltaSeconds (`self.Rotation Time`)))
  (`self.K2_SetActorLocation` (`KismetMathLibrary.VLerp` (`self.StartLocation`) (`self.EndLocation`) (/ (`self.Current Time`) (`self.Rotation Time`))))
  (if (>= (`self.Current Time`) (`self.Rotation Time`))
    (`self.SetActorTickEnabled` false)))

(fn `UserConstructionScript`)