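; BP_Puzzle is a rotation-code puzzle actor that opens or closes a secret passage on its linked Door.
; InteractwithPuzzles yaws the given mesh left or right by RotateValue, prints the rotation, then runs CheckCode.
; CheckCode compares that mesh's relative yaw to its Code entry with a small tolerance, opening the passage only when all CodeIsGood flags are true.
; Box overlap shows an interaction widget for the third-person character and removes it on end overlap.
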(event `/Game/FinalProject/InteractWithPuzzles.InteractWithPuzzles`
  (params (Components :type "PrimitiveComponent Object Reference") (RotateLeft :type Boolean))
  (`self.Rotate` Components RotateLeft))

(event `self.Box.OnComponentBeginOverlap`
  (params (OverlappedComponent :type "PrimitiveComponent Object Reference") (OtherActor :type "Actor Object Reference") (OtherComp :type "PrimitiveComponent Object Reference") (OtherBodyIndex :type Integer) (bFromSweep :type Boolean) (SweepResult :type "HitResult Structure (by ref)"))
  (cast `/Game/FinalProject/BP_ThirdPersonCharacter` OtherActor)
  (bind _returnvalue (`|CreateWidget` "/Game/FinalProject/InteractPuzzle_Widget.InteractPuzzle_Widget_C"))
  (`UserWidget.AddToViewport` _returnvalue 0))

(event `self.Box.OnComponentEndOverlap`
  (params (OverlappedComponent :type "PrimitiveComponent Object Reference") (OtherActor :type "Actor Object Reference") (OtherComp :type "PrimitiveComponent Object Reference") (OtherBodyIndex :type Integer))
  (`Widget.RemoveFromParent` (stale `self.Box.OnComponentBeginOverlap` _returnvalue)))

(fn `CheckCode`
  (params (Components :type "PrimitiveComponent Object Reference"))
  (locals (SelectedMash :type Integer) (LocalFailed :type Boolean))
  (bind _door (`self.Door`))
  (bind (_relativerotation_roll _relativerotation_pitch _relativerotation_yaw) (`KismetMathLibrary.BreakRotator` (`SceneComponent.RelativeRotation` Components)))
  (if (== Components (`self.StaticMesh`))
    (set `local.SelectedMash` 0)
    (`KismetArrayLibrary.Array_Set` (`self.CodeIsGood`) (`local.SelectedMash`) (`KismetMathLibrary.NearlyEqual_FloatFloat` (`|GetArrayItem` (`self.Code`) (`local.SelectedMash`)) _relativerotation_yaw 1.0) :!label _label)
    (for _array_element (`self.CodeIsGood`)
      (if (not _array_element)
        (set `local.LocalFailed` true)
        (break)))
    (if (`local.LocalFailed`)
      (`/Game/FinalProject/BP_Door.CloseSecretGeçiş` _door)
      (else
        (`/Game/FinalProject/BP_Door.OpenSecretGeçiş` _door)))
    (elif (== Components (`self.StaticMesh1`))
      (set `local.SelectedMash` 1)
      (goto _label)
      (elif (== Components (`self.StaticMesh2`))
        (set `local.SelectedMash` 2)
        (goto _label)))))

(fn `Rotate`
  (params (Components :type "PrimitiveComponent Object Reference") (RotateLeft :type Boolean))
  (if RotateLeft
    (`SceneComponent.K2_AddRelativeRotation` Components (`KismetMathLibrary.MakeRotator` 0.0 0.0 (* (`self.RotateValue`) -1.0)) false false)
    (else
      (`SceneComponent.K2_AddRelativeRotation` Components (`KismetMathLibrary.MakeRotator` 0.0 0.0 (`self.RotateValue`)) false false)))
  (`KismetSystemLibrary.PrintString` (`KismetStringLibrary.Conv_RotatorToString` (`SceneComponent.RelativeRotation` Components)))
  (`self.CheckCode` Components))

(fn `UserConstructionScript`)